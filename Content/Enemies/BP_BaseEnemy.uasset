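; BP_BaseEnemy is a base enemy actor that advances steadily along negative world X and can be killed by damage.
; Tick applies a frame-rate-independent world offset without sweep, so movement ignores blocking collision.
; AnyDamage writes reduced Health into the Stats struct, then destroys the actor if that value minus Damage again is zero or below.
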(event EventBeginPlay)

(event Collision|EventActorBeginOverlap
  (params (OtherActor :type Actor%20Object%20Reference)))

(event EventTick
  (params (DeltaSeconds :type Float%20%28single-precision%29))
  (Transformation|AddActorWorldOffset (Math|Vector|MakeVector (* DeltaSeconds -5e+01) 0.0 0.0)))

(event Game|Damage|EventAnyDamage
  (params (Damage :type Float%20%28single-precision%29) (DamageType :type Damage%20Type%20Object%20Reference) (InstigatedBy :type Controller%20Object%20Reference) (DamageCauser :type Actor%20Object%20Reference))
  (bind _stats (Variables|Default|GetStats))
  (bind _health (Utilities|Struct|BreakF_EnemyStatsStruct _stats))
  (bind _returnvalue (- _health Damage))
  (Utilities|Struct|SetmembersinF_EnemyStatsStruct _stats _returnvalue)
  (if (<= _returnvalue 0.0)
    (Actor|DestroyActor)))

(fn ConstructionScript)