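; BP_BaseRoot is a base root Blueprint with a Paper2D sprite, apparently an early AI root pathing prototype.
; On BeginPlay it converts a vector array into world-space points using a fixed multiplier and the sprite's rotation, scale and location.
; It draws temporary debug points and stores unique results in VectorsInWorldspace.
; It then runs a persistently drawn Visibility line trace between the first two points, leaving the result unused.
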(event EventBeginPlay
  (bind _papersprite (Variables|Default|GetPaperSprite))
  (bind _vectorsinworldspace (Variables|Default|GetVectorsInWorldspace))
  (for _array_element (Variables|Default|GetVector)
    (Rendering|Debug|DrawDebugPoint (+ (* (Math|Vector|RotateVector (* _array_element "10.000000,10.000000,10.000000") (Transformation|GetWorldRotation _papersprite)) (Transformation|GetWorldScale _papersprite)) (Transformation|GetWorldLocation _papersprite)) 1e+01 "(R=1.000000,G=0.511483,B=0.000000,A=1.000000)" 2e+01)
    (Utilities|Array|AddUnique (Variables|Default|GetVectorsInWorldspace) (+ (* (Math|Vector|RotateVector (* _array_element "10.000000,10.000000,10.000000") (Transformation|GetWorldRotation _papersprite)) (Transformation|GetWorldScale _papersprite)) (Transformation|GetWorldLocation _papersprite))))
  (Collision|LineTraceByChannel (Utilities|Array|Get(acopy) _vectorsinworldspace) (Utilities|Array|Get(acopy) _vectorsinworldspace 1) "TraceTypeQuery1" false 0 "Persistent"))

(event Collision|EventActorBeginOverlap
  (params (OtherActor :type Actor%20Object%20Reference)))

(event EventTick
  (params (DeltaSeconds :type Float%20%28single-precision%29)))

(fn ConstructionScript)