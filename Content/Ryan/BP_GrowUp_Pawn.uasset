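; Pawn for the beetroot pumping minigame, opened from a main menu widget, where alternating A and D presses grow the beetroot.
; A raises the pump; D lowers it, increments PumpLevel and grows the beetroot through timelines and mesh swaps, while key prompts alternate.
; The first D pump dismisses the tutorial and starts a ten-second timer.
; GameOver then either prints an insult or saves Size to BP_BeetrootInstance and fades toward ShowerGame.
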(event Custom|Game%20Over
  (if (< (Variables|Default|GetPump_Level) 20)
    (Development|PrintString "FUCKING NOOB")
    (else
      (bind _asbp_beetroot_instance (Utilities|Casting|CastToBP_BeetrootInstance (Game|GetGameInstance)))
      (Default|StatstoAdd _asbp_beetroot_instance 0 (Variables|Default|GetPump_Level))
      (Variables|/Game/Ryan/StatsStruct/BP_BeetrootInstance.BP_BeetrootInstance_C|SetLevel%20To%20Travel%20To _asbp_beetroot_instance "ShowerGame")
      (bind _returnvalue (UserInterface|CreateWidget "/Game/Ryan/UI_FadeToBlack.UI_FadeToBlack_C"))
      (UserInterface|Viewport|AddtoViewport _returnvalue 0))))

(event Custom|Start
  ;[1 1 1] ON start game
  (Variables|Default|SetInput%20enabled true)
  (Variables|/Script/Engine.PlayerController|SetbShowMouseCursor (Game|GetPlayerController 0) false)
  (Input|EnableInput (Game|GetPlayerController 0))
  (bind _returnvalue (UserInterface|CreateWidget "/Game/Ryan/Shower/UI_ShowerTutorial.UI_ShowerTutorial_C" 0 "Pump your beetroot"))
  (bind _output_get (Variables|Default|SetDelightful _returnvalue))
  (UserInterface|Viewport|AddtoViewport _output_get 0)
  (Rendering|SetVisibility (Variables|Default|GetD) true false))

(event Collision|EventActorBeginOverlap
  (params (OtherActor :type Actor%20Object%20Reference)))

(event EventBeginPlay
  (bind _returnvalue (UserInterface|CreateWidget "/Game/Ryan/UI_MainMenu.UI_MainMenu_C"))
  (EventDispatchers|BindEventtoStartGame _returnvalue (delegate Custom|Start))
  (UserInterface|Viewport|AddtoViewport _returnvalue 0)
  (Variables|/Script/Engine.PlayerController|SetbShowMouseCursor (Game|GetPlayerController 0) true)
  (Rendering|SetVisibility (Variables|Default|GetD) false false))

(event Input|KeyboardEvents|A
  (params (Key :type Key%20Structure :default "None"))
  (:Pressed
    (if (Variables|Default|GetInput%20enabled)
      (if (Variables|Default|GetA?)
        (bind _returnvalue (Audio|SpawnSound2D "/Game/Ryan/PumpingRoots/Pump_Up.Pump_Up" 0.2 1.0 0.0 0))
        (Variables|Default|SetA? false)
        (Utilities|FlowControl|Sequence
          (:then_0
            (goto _label Reset))
          (:then_1
            (bind _newtrack_0 (Timeline|Timeline_0 PlayFromStart)
              (:Update
                (Transformation|SetRelativeLocation (Variables|Default|GetPump) (Math|Vector|Lerp(Vector) "0, 0, 0" "0, 0,40.000000" _newtrack_0) false false)
                (Utilities|FlowControl|DoOnce false :!label _label
                  (:Completed
                    (Rendering|SetVisibility (Variables|Default|GetA) false false)
                    (Rendering|SetVisibility (Variables|Default|GetD) true false)))))))))))

(event Input|KeyboardEvents|D
  (params (Key :type Key%20Structure :default "None"))
  (bind _beetroot (Variables|Default|GetBeetRoot))
  (:Pressed
    (if (Variables|Default|GetInput%20enabled)
      (if (not (Variables|Default|GetA?))
        (bind _returnvalue (Audio|SpawnSound2D "/Game/Ryan/PumpingRoots/Pump_Down.Pump_Down" 0.2 1.0 0.0 0))
        (Variables|Default|SetA? true)
        (Utilities|FlowControl|Sequence
          (:then_0
            ;[1 1 1] WHERE TO KILL WIDGET
            (Utilities|FlowControl|DoOnce false
              (:Completed
                (Default|DieWidget (Variables|Default|GetDelightful))
                (bind _returnvalue_2 (UserInterface|CreateWidget "/Game/Ryan/Shower/UI_10SecondTimer.UI_10SecondTimer_C"))
                (UserInterface|Viewport|AddtoViewport _returnvalue_2 0)
                (Utilities|Time|SetTimerbyEvent (delegate Custom|Game%20Over) 1e+01))))
          (:then_1
            (Math|Integer|IncrementInt (Variables|Default|GetPump_Level)
              (:%20%20
                (Utilities|FlowControl|Sequence
                  (:then_0
                    (goto _label Reset))
                  (:then_1
                    (bind _newtrack_0 (Timeline|Timeline_1 PlayFromStart)
                      (:Update
                        (Transformation|SetWorldScale3D _beetroot (Math|Vector|Lerp(Vector) (Variables|Default|GetScale) (+ (Variables|Default|GetScale) 0.1) _newtrack_0))
                        (Utilities|FlowControl|DoOnce false :!label _label
                          (:Completed
                            (Variables|Default|SetScale (+ (Variables|Default|GetScale) 0.1))
                            (if (>= (.X (Math|Vector|BreakVector (Variables|Default|GetScale))) 2.0)
                              (if (>= (.X (Math|Vector|BreakVector (Variables|Default|GetScale))) 2.1)
                                (Utilities|FlowControl|DoOnce false
                                  (:Completed
                                    (Components|StaticMesh|SetStaticMesh _beetroot "/Game/PolygonFarm/Meshes/Plants/SM_Prop_Beetroot_01_L.SM_Prop_Beetroot_01_L")
                                    (Variables|Default|SetScale "1.600000,1.600000,1.600000")
                                    (Transformation|SetWorldScale3D _beetroot "1.500000,1.500000,1.500000")))
                                (else
                                  (Utilities|FlowControl|DoOnce false
                                    (:Completed
                                      (Components|StaticMesh|SetStaticMesh _beetroot "/Game/PolygonFarm/Meshes/Plants/SM_Prop_Beetroot_01_M.SM_Prop_Beetroot_01_M")
                                      (Variables|Default|SetScale "1.300000,1.300000,1.300000")
                                      (Transformation|SetWorldScale3D _beetroot "1.200000,1.200000,1.200000")))))))))))))))
          (:then_2
            (Utilities|FlowControl|Sequence
              (:then_0
                (goto _label_2 Reset))
              (:then_1
                (bind _newtrack_0_2 (Timeline|Timeline_2 PlayFromStart)
                  (:Update
                    (Transformation|SetRelativeLocation (Variables|Default|GetPump) (Math|Vector|Lerp(Vector) "0, 0,40.000000" "0, 0, 0" _newtrack_0_2) false false)
                    (Utilities|FlowControl|DoOnce false :!label _label_2
                      (:Completed
                        (Rendering|SetVisibility (Variables|Default|GetA) true false)
                        (Rendering|SetVisibility (Variables|Default|GetD) false false)))))))))))))

(fn ConstructionScript)