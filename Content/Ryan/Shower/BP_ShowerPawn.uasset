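; Pawn for a timed shower minigame in which the player sweeps a cursor-following sprite to pop bubbles.
; Tick moves the sprite to the visibility trace under the hidden cursor, and box overlaps destroy Bubble-tagged actors to add score.
; BeginPlay shows countdown and tutorial widgets, runs the delayed play window, prints the result, awards score-based Cleanliness through BP_BeetrootInstance, then opens TheLevel.
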(event OnComponentBeginOverlap(Box)
  (params (OverlappedComponent :type Primitive%20Component%20Object%20Reference) (OtherActor :type Actor%20Object%20Reference) (OtherComp :type Primitive%20Component%20Object%20Reference) (OtherBodyIndex :type Integer) (bFromSweep :type Boolean) (SweepResult :type Hit%20Result%20Structure%20%28by%20ref%29))
  (if (Actor|ActorHasTag OtherActor "Bubble")
    (Actor|DestroyActor OtherActor)
    (Math|Integer|IncrementInt (Variables|Default|GetScore))))

(event EventBeginPlay
  (bind _returnvalue (Game|GetPlayerController 0))
  (bind _score (Variables|Default|GetScore))
  (bind _returnvalue_2 (> _score 99))
  (Utilities|FlowControl|Sequence
    (:then_0
      (bind _returnvalue_3 (UserInterface|CreateWidget "/Game/Ryan/Shower/UI_Countdown.UI_Countdown_C"))
      (UserInterface|Viewport|AddtoViewport _returnvalue_3 0))
    (:then_1
      (bind _returnvalue_4 (UserInterface|CreateWidget "/Game/Ryan/Shower/UI_ShowerTutorial.UI_ShowerTutorial_C"))
      (UserInterface|Viewport|AddtoViewport _returnvalue_4 0)
      (Variables|/Script/Engine.PlayerController|SetbShowMouseCursor _returnvalue false)
      (Variables|/Script/Engine.PlayerController|SetbEnableMouseOverEvents _returnvalue true)
      (Transformation|SetWorldLocation (Variables|Default|GetPaperSprite) "0, 0, 0" true false)
      (Utilities|FlowControl|Delay 3.0)
      (Variables|Default|SetMouse%20movement true)
      (Utilities|FlowControl|Delay 1e+01)
      (Development|PrintString (Utilities|String|ToString(Integer) _score) true true "(R=0.000000,G=0.660000,B=1.000000,A=1.000000)" 99.0)
      (Development|PrintString (select _returnvalue_2 "Epic" "Loser") true true "(R=0.000000,G=0.660000,B=1.000000,A=1.000000)" 99.0)
      (bind _asbp_beetroot_instance (Utilities|Casting|CastToBP_BeetrootInstance (Game|GetGameInstance)))
      (Default|StatstoAdd _asbp_beetroot_instance (select _returnvalue_2 5 1))
      (Utilities|FlowControl|Delay 1.0)
      (Game|OpenLevel(byName) "TheLevel"))))

(event EventTick
  (params (DeltaSeconds :type Float%20%28single-precision%29))
  (if (Variables|Default|GetMouse%20movement)
    (Transformation|SetWorldLocation (Variables|Default|GetPaperSprite) (.ImpactPoint (Collision|BreakHitResult (.HitResult (Game|Player|GetHitResultUnderCursorbyChannel (Game|GetPlayerController 0) "TraceTypeQuery1" true)))) true false)))

(fn ConstructionScript)