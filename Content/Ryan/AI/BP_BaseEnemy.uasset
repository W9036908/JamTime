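; BP_BaseEnemy is an early base enemy actor with only debug distance logic in place.
; On BeginPlay it stores the distance from StartLocation to TargetLocation, then prints the root component's remaining distance to the target as a fraction of it.
; Tick and the construction script are empty, and the SetWorldLocation and vector Lerp nodes are unconnected, so the actor does not move.
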(event EventBeginPlay
  (Variables|Default|SetDestinationDistance (Math|Vector|Distance(Vector) (Variables|Default|GetStartLocation) (Variables|Default|GetTargetLocation)))
  (Development|PrintString (Utilities|String|ToString(Float) (/ (Math|Vector|Distance(Vector) (Transformation|GetWorldLocation (Variables|Default|GetDefaultSceneRoot)) (Variables|Default|GetTargetLocation)) (Variables|Default|GetDestinationDistance)))))

(event Collision|EventActorBeginOverlap
  (params (OtherActor :type Actor%20Object%20Reference)))

(event EventTick
  (params (DeltaSeconds :type Float%20%28single-precision%29)))

(fn ConstructionScript)