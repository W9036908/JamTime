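; BP_BeetrootInstance holds a beetroot's running stats for Cleanliness, Size and Tastiness in an FStats struct.
; The StatsToAdd event stores incoming values as a pending FStats, overwriting the previous one.
; The Addstats event adds that pending struct field by field into BeatStats, without clearing it afterward.
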(event Custom|StatsToAdd
  (params (Cleanliness :type Integer) (Size :type Integer) (Tastiness :type Integer))
  (Variables|Default|SetStats%20to%20add (Utilities|Struct|MakeF_Stats Cleanliness Size Tastiness)))

(event Custom|Add%20stats
  (bind _stats_to_add (Variables|Default|GetStats%20to%20add))
  (bind (_cleanliness _size _tastiness) (Utilities|Struct|BreakF_Stats _stats_to_add))
  (Variables|Default|SetBeatStats (Utilities|Struct|MakeF_Stats (+ _cleanliness (.Cleanliness (Utilities|Struct|BreakF_Stats (Variables|Default|GetBeatStats)))) (+ _size (.Size (Utilities|Struct|BreakF_Stats (Variables|Default|GetBeatStats)))) (+ _tastiness (.Tastiness (Utilities|Struct|BreakF_Stats (Variables|Default|GetBeatStats)))))))