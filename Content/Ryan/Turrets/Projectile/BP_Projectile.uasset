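; BP_Projectile is a turret projectile that damages actors tagged Enemy.
; On BeginPlay it sets its ProjectileMovement velocity from the speed in ProjectileStats, rotated to the actor's facing.
; On overlap with an Enemy-tagged actor it applies the damage from ProjectileStats and destroys itself.
; Other overlaps are ignored, and the Hit event does nothing.
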(event EventTick
  (params (DeltaSeconds :type Float%20%28single-precision%29)))

(event Collision|EventHit
  (params (MyComp :type Primitive%20Component%20Object%20Reference) (Other :type Actor%20Object%20Reference) (OtherComp :type Primitive%20Component%20Object%20Reference) (bSelfMoved :type Boolean) (HitLocation :type Vector :default "0, 0, 0") (HitNormal :type Vector :default "0, 0, 0") (NormalImpulse :type Vector :default "0, 0, 0") (Hit :type Hit%20Result%20Structure%20%28by%20ref%29)))

(event Collision|EventActorBeginOverlap
  (params (OtherActor :type Actor%20Object%20Reference))
  (if (Actor|ActorHasTag OtherActor "Enemy")
    (Game|Damage|ApplyDamage OtherActor (.Damage (Utilities|Struct|BreakF_ProjectileStats (Variables|Default|GetProjectileStats))) 0 0)
    (Actor|DestroyActor)))

(event EventBeginPlay
  (Variables|/Script/Engine.MovementComponent|SetVelocity (Variables|Default|GetProjectileMovement) (Math|Vector|RotateVector (Math|Vector|MakeVector (.Speed (Utilities|Struct|BreakF_ProjectileStats (Variables|Default|GetProjectileStats))) 0.0 0.0) (Transformation|GetActorRotation))))

(fn ConstructionScript)