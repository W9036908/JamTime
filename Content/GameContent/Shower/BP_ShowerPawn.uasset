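; Player pawn for the shower minigame, where the mouse is used to clean the beetroot.
; BeginPlay shows countdown and tutorial widgets, then after a short delay hides the cursor and starts a timed round.
; Tick snaps the sprite to the cursor trace's impact point, and Box overlaps destroy Bubble-tagged actors to raise Score.
; When time expires, Score goes to the game instance as Cleanliness, Treadmill becomes the next level, and a fade widget appears.
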(event OnComponentBeginOverlap(Box)
  (params (OverlappedComponent :type Primitive%20Component%20Object%20Reference) (OtherActor :type Actor%20Object%20Reference) (OtherComp :type Primitive%20Component%20Object%20Reference) (OtherBodyIndex :type Integer) (bFromSweep :type Boolean) (SweepResult :type Hit%20Result%20Structure%20%28by%20ref%29))
  (if (Actor|ActorHasTag OtherActor "Bubble")
    (Actor|DestroyActor OtherActor)
    (Math|Integer|IncrementInt (Variables|Default|GetScore))))

(event EventBeginPlay
  (bind _returnvalue (Game|GetPlayerController 0))
  (Utilities|FlowControl|Sequence
    (:then_0
      (bind _returnvalue_2 (UserInterface|CreateWidget "/Game/GameContent/Shower/UI_Countdown.UI_Countdown_C"))
      (UserInterface|Viewport|AddtoViewport _returnvalue_2 0)
      (Variables|/Script/Engine.PlayerController|SetbShowMouseCursor (Game|GetPlayerController 0) true))
    (:then_1
      (bind _returnvalue_3 (UserInterface|CreateWidget "/Game/GameContent/Shower/UI_ShowerTutorial.UI_ShowerTutorial_C" 0 "Use the mouse to clean the beetroot" true))
      (UserInterface|Viewport|AddtoViewport _returnvalue_3 0)
      (Variables|/Script/Engine.PlayerController|SetbShowMouseCursor _returnvalue true)
      (Variables|/Script/Engine.PlayerController|SetbEnableMouseOverEvents _returnvalue true)
      (Transformation|SetWorldLocation (Variables|Default|GetPaperSprite) "0, 0, 0" true false)
      (Utilities|FlowControl|Delay 3.0)
      (Variables|/Script/Engine.PlayerController|SetbShowMouseCursor (Game|GetPlayerController 0) false)
      (Variables|Default|SetMouse%20movement true)
      (Utilities|FlowControl|Delay 1e+01)
      (bind _asbp_beetroot_instance (Utilities|Casting|CastToBP_BeetrootInstance (Game|GetGameInstance)))
      (Default|StatstoAdd _asbp_beetroot_instance (Variables|Default|GetScore))
      (Variables|/Game/GameContent/StatsStruct/BP_BeetrootInstance.BP_BeetrootInstance_C|SetLevel%20To%20Travel%20To _asbp_beetroot_instance "Treadmill")
      (bind _returnvalue_4 (UserInterface|CreateWidget "/Game/GameContent/UI_FadeToBlack.UI_FadeToBlack_C"))
      (UserInterface|Viewport|AddtoViewport _returnvalue_4 0))))

(event EventTick
  (params (DeltaSeconds :type Float%20%28single-precision%29))
  (if (Variables|Default|GetMouse%20movement)
    (Transformation|SetWorldLocation (Variables|Default|GetPaperSprite) (.ImpactPoint (Collision|BreakHitResult (.HitResult (Game|Player|GetHitResultUnderCursorbyChannel (Game|GetPlayerController 0) "TraceTypeQuery1" true)))) true false)))

(fn ConstructionScript)